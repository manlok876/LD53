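; BP_PostmanController is the player controller that turns Enhanced Input into movement, look and jump for the Postman character.
; BeginPlay adds the IMC_Postman mapping context, and possession caches the pawn as a Character for the validity-checked jump.
; Move input is rotated by control yaw into camera-relative movement on the controlled pawn.
; Look input, scaled by CameraSpeedMultiplier, is added directly to control rotation pitch and yaw.
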(event Input|EnhancedActionEvents|EnhancedInputActionIA_Move
  (params (ActionValue :type Vector%202D%20Structure) (ElapsedSeconds :type Float%20%28double-precision%29) (TriggeredSeconds :type Float%20%28double-precision%29) (InputAction :type Input%20Action%20Object%20Reference :default "/Game/Player/Input/IA_Move.IA_Move"))
  (:Triggered
    (Pawn|Input|AddMovementInput (Pawn|GetControlledPawn) (Math|Conversions|ToVector(Vector2D) (Class|KismetMathLibrary|GetRotated2D ActionValue (.Yaw (Math|Rotator|BreakRotator (Pawn|GetControlRotation :!class /Script/Engine.Controller))))) 1.0 false)))

(event Input|EnhancedActionEvents|EnhancedInputActionIA_Look
  (params (ActionValue :type Vector%202D%20Structure) (ElapsedSeconds :type Float%20%28double-precision%29) (TriggeredSeconds :type Float%20%28double-precision%29) (InputAction :type Input%20Action%20Object%20Reference :default "/Game/Player/Input/IA_Look.IA_Look"))
  (bind _returnvalue (Pawn|GetControlRotation :!class /Script/Engine.Controller))
  (bind _cameraspeedmultiplier (Variables|Input|GetCameraSpeedMultiplier))
  (bind (_roll _pitch _yaw) (Math|Rotator|BreakRotator _returnvalue))
  (bind _returnvalue_2 (* ActionValue (Math|Vector2D|MakeVector2D _cameraspeedmultiplier _cameraspeedmultiplier)))
  (bind (_x _y) (Math|Vector2D|BreakVector2D _returnvalue_2))
  (:Triggered
    (Pawn|SetControlRotation (Math|Rotator|MakeRotator _roll (+ _pitch _y) (+ _yaw _x)))))

(event Input|EnhancedActionEvents|EnhancedInputActionIA_Jump
  (params (ActionValue :type Boolean) (ElapsedSeconds :type Float%20%28double-precision%29) (TriggeredSeconds :type Float%20%28double-precision%29) (InputAction :type Input%20Action%20Object%20Reference :default "/Game/Player/Input/IA_Jump.IA_Jump"))
  (:Triggered
    (bind _postmancharacter (Variables|Default|GetPostmanCharacter)
      (:then
        (Character|Jump _postmancharacter))
      (:else))))

(event EventBeginPlay
  (Input|AddMappingContext (PlayerController|LocalPlayerSubsystems|GetEnhancedInputLocalPlayerSubsystem) "/Game/Player/Input/IMC_Postman.IMC_Postman" 0 "(bIgnoreAllPressedKeysUntilRelease=True,bForceImmediately=False)"))

(event EventTick
  (params (DeltaSeconds :type Float%20%28single-precision%29)))

(event EventPossess
  (params (PossessedPawn :type Pawn%20Object%20Reference))
  (bind _ascharacter (Utilities|Casting|CastToCharacter PossessedPawn))
  (Variables|Default|SetPostmanCharacter _ascharacter))

(fn ConstructionScript)