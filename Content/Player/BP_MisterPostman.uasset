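; Player postman pawn that picks up, carries and throws BP_Package actors.
; Each tick, a camera line trace finds a package to show the take prompt, while a PhysicsHandle holds any grabbed box along the view direction.
; IA_Take grabs, or when already holding charges a throw on a colored progress bar and launches on release, using gates to separate the two presses.
; Mouse wheel adjusts the clamped hold distance.
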(event Custom|CheckTake
  (bind _returnvalue (Game|GetPlayerCameraManager 0))
  (bind _returnvalue_2 (Camera|GetCameraLocation _returnvalue))
  (Utilities|IsValid (Class|PhysicsHandleComponent|GetGrabbedComponent (Variables|Default|GetPhysicsHandle))
    (:Is%20Valid
      (Default|ShowTake (Variables|Default|GetPlayerScreenWidget) false)
      (Variables|Default|SetLookAtPackage 0))
    (:Is%20Not%20Valid
      (bind (_outhit _returnvalue_3) (Collision|LineTraceByChannel _returnvalue_2 (+ _returnvalue_2 (* (Math|Vector|GetForwardVector (Camera|GetCameraRotation _returnvalue)) (Math|Conversions|ToVector(Float) (Variables|Default|GetTraceLength)))) "TraceTypeQuery1" false 0 "None"))
      (if _returnvalue_3
        (bind _asbp_package (Utilities|Casting|CastToBP_Package (.HitActor (Collision|BreakHitResult _outhit)))
          (:then
            (Default|ShowTake (Variables|Default|GetPlayerScreenWidget) true)
            (Variables|Default|SetLookAtPackage _asbp_package))
          (:CastFailed
            (Default|ShowTake (Variables|Default|GetPlayerScreenWidget) false :!label _label)
            (Variables|Default|SetLookAtPackage 0)))
        (else
          (goto _label))))))

(event Input|EnhancedActionEvents|EnhancedInputActionIA_Take
  (params (ActionValue :type Boolean) (ElapsedSeconds :type Float%20%28double-precision%29) (TriggeredSeconds :type Float%20%28double-precision%29) (InputAction :type Input%20Action%20Object%20Reference :default "/Game/Player/Input/IA_Take.IA_Take"))
  (bind _playerscreenwidget (Variables|Default|GetPlayerScreenWidget))
  (bind _playerscreenwidget_2 (Variables|Default|GetPlayerScreenWidget))
  (bind _lookatpackage (Variables|Default|GetLookAtPackage))
  (bind _box (Variables|/Game/Blueprints/Package/BP_Package.BP_Package_C|GetBox _lookatpackage))
  (bind _progressbar_0 (Variables|/Game/Player/PlayerHUD/WBP_PlayerHUD.WBP_PlayerHUD_C|GetProgressBar_0 _playerscreenwidget))
  (bind _progressbar_0_2 (Variables|/Game/Player/PlayerHUD/WBP_PlayerHUD.WBP_PlayerHUD_C|GetProgressBar_0 _playerscreenwidget_2))
  (:Triggered
    (Utilities|FlowControl|Gate true :!label _label
      (:Exit
        (Variables|Throw|SetThrowStrange (+ (Variables|Throw|GetThrowStrange) (Utilities|Time|GetWorldDeltaSeconds)))
        (Variables|/Script/UMG.Widget|SetVisibility _progressbar_0_2 "Visible")
        (Progress|SetPercent _progressbar_0_2 (Math|Float|MapRangeClamped (Variables|Throw|GetThrowStrange) 0.0 (Variables|Throw|GetThrowTimeMax) 0.0 1.0))
        (Class|ProgressBar|SetFillColorandOpacity (Variables|/Game/Player/PlayerHUD/WBP_PlayerHUD.WBP_PlayerHUD_C|GetProgressBar_0 (Variables|Default|GetPlayerScreenWidget)) (Math|Color|Lerp(LinearColor) "(R=0.000000,G=1.000000,B=0.137825,A=1.000000)" "(R=1.000000,G=0.000000,B=0.000000,A=1.000000)" (Math|Float|MapRangeClamped (Variables|Throw|GetThrowStrange) 0.0 (Variables|Throw|GetThrowTimeMax) 0.0 1.0))))))
  (:Started
    (Utilities|IsValid (Class|PhysicsHandleComponent|GetGrabbedComponent (Variables|Default|GetPhysicsHandle))
      (:Is%20Valid
        (Utilities|FlowControl|Sequence
          (:then_0
            (goto _label Open))
          (:then_1
            (goto _label_2 Open))))
      (:Is%20Not%20Valid
        (Utilities|FlowControl|Sequence
          (:then_0
            (Utilities|IsValid _lookatpackage
              (:Is%20Valid
                (Physics|Components|PhysicsHandle|GrabComponentatLocationwithRotation (Variables|Default|GetPhysicsHandle) _box "None" (Transformation|GetWorldLocation _box) (Transformation|GetWorldRotation _box)))))
          (:then_1
            (goto _label_2 Close))
          (:then_2
            (goto _label Close))))))
  (:Completed
    (Utilities|FlowControl|Gate true :!label _label_2
      (:Exit
        (Utilities|IsValid (Class|PhysicsHandleComponent|GetGrabbedComponent (Variables|Default|GetPhysicsHandle))
          (:Is%20Valid
            (Physics|AddImpulse (Class|PhysicsHandleComponent|GetGrabbedComponent (Variables|Default|GetPhysicsHandle)) (* (Math|Vector|GetForwardVector (Camera|GetCameraRotation (Game|GetPlayerCameraManager 0))) (Math|Float|MapRangeClamped (Variables|Throw|GetThrowStrange) 0.0 (Variables|Throw|GetThrowTimeMax) 0.0 (Variables|Throw|GetThrowImpulseMax))) "None" false)
            (Physics|Components|PhysicsHandle|ReleaseComponent (Variables|Default|GetPhysicsHandle))
            (Variables|GrabOffset|SetGrabOffset 0.0)
            (Variables|Throw|SetThrowStrange 0.0)
            (Variables|/Script/UMG.Widget|SetVisibility _progressbar_0 "Collapsed")
            (Progress|SetPercent _progressbar_0 0.0)))))))

(event Input|EnhancedActionEvents|EnhancedInputActionIA_MouseWheel
  (params (ActionValue :type Float%20%28double-precision%29) (ElapsedSeconds :type Float%20%28double-precision%29) (TriggeredSeconds :type Float%20%28double-precision%29) (InputAction :type Input%20Action%20Object%20Reference :default "/Game/Player/Input/IA_MouseWheel.IA_MouseWheel"))
  (:Triggered
    (Variables|GrabOffset|SetGrabOffset (Math|Float|Clamp(Float) (+ (Variables|GrabOffset|GetGrabOffset) (* ActionValue (Variables|GrabOffset|GetGrabOffsetMultiply))) (Variables|GrabOffset|GetMinGramOffset) (Variables|GrabOffset|GetMaxGrabOffset)))))

(event EventBeginPlay
  (bind _returnvalue (UserInterface|CreateWidget "/Game/Player/PlayerHUD/WBP_PlayerHUD.WBP_PlayerHUD_C" (Game|GetPlayerController 0)))
  (bind _output_get (Variables|Default|SetPlayerScreenWidget _returnvalue))
  (UserInterface|Viewport|AddtoViewport _output_get 0))

(event EventTick
  (params (DeltaSeconds :type Float%20%28single-precision%29))
  (bind _grablocation (Variables|Default|GetGrabLocation))
  (CallFunction|CheckTake)
  (Class|PhysicsHandleComponent|SetTargetLocationandRotation (Variables|Default|GetPhysicsHandle) (+ (Transformation|GetWorldLocation _grablocation) (* (Math|Vector|GetForwardVector (Camera|GetCameraRotation (Game|GetPlayerCameraManager 0))) (Math|Conversions|ToVector(Float) (Variables|GrabOffset|GetGrabOffset)))) (Transformation|GetWorldRotation _grablocation)))

(fn ConstructionScript)