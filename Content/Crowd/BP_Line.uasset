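; BP_Line is a spline-based waiting line for crowd pawns, where each spline point is a numbered place to stand.
; Pawns register to receive their index and world location, and can query their number, any place's location, or the line length.
; Unregistering removes a pawn from the ordered array and fires LineUpdate, as the indices behind it shift.
; The construction script rebuilds "Person N" text labels above each point, hidden in game.
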(fn ConstructionScript
  (bind _textrendercomponents (Variables|TextSetting|GetTextRenderComponents))
  (for _array_element _textrendercomponents
    (Components|DestroyComponent _array_element))
  (Utilities|Array|Clear _textrendercomponents)
  (for _index (range 0 (- (Spline|GetNumberOfSplinePoints (Variables|Default|GetSpline)) 1))
    (bind _returnvalue (AddComponent|AddTextRenderComponent true (Math|Transform|MakeTransform (+ (.Location (Math|Transform|BreakTransform (Spline|GetTransformatSplinePoint (Variables|Default|GetSpline) _index "World" false))) (Math|Vector|MakeVector 0.0 0.0 (Variables|TextSetting|GetTextHeight))) (.Rotation (Math|Transform|BreakTransform (Spline|GetTransformatSplinePoint (Variables|Default|GetSpline) _index "World" false))) (.Scale (Math|Transform|BreakTransform (Spline|GetTransformatSplinePoint (Variables|Default|GetSpline) _index "World" false))))))
    (Utilities|Array|Add (Variables|TextSetting|GetTextRenderComponents) _returnvalue)
    (Rendering|Components|TextRender|SetText _returnvalue (Utilities|Text|FormatText "Person {Num}" _index))
    (Rendering|Components|TextRender|SetHorizontalAlignment _returnvalue "EHTA_Center")
    (Rendering|Components|TextRender|SetTextRenderColor _returnvalue (Variables|TextSetting|GetTextColor))
    (Development|SetHiddeninGame _returnvalue true false)))

(fn RegisterinLine
  (params (Pawn :type Pawn%20Object%20Reference%20%28by%20ref%29))
  (bind _returnvalue (Utilities|Array|Add (Variables|Default|GetPawnsInLine) Pawn))
  (return _returnvalue (.Location (Math|Transform|BreakTransform (Spline|GetTransformatSplinePoint (Variables|Default|GetSpline) _returnvalue "World" false)))))

(fn UnregisterfromLine
  (params (Pawn :type Pawn%20Object%20Reference%20%28by%20ref%29))
  (bind _pawnsinline (Variables|Default|GetPawnsInLine))
  (bind _returnvalue (Utilities|Array|FindItem _pawnsinline Pawn))
  (LocalVariables|SetTempNumber _returnvalue)
  (if (not (== _returnvalue -1))
    (Utilities|Array|RemoveItem _pawnsinline Pawn)
    (Default|CallLineUpdate self)))

(fn GetLineLength
  (return (Utilities|Array|Length (Variables|Default|GetPawnsInLine))))

(fn GetPlaceatNumber
  (params (Number :type Integer))
  (return (.Location (Math|Transform|BreakTransform (Spline|GetTransformatSplinePoint (Variables|Default|GetSpline) Number "World" false)))))

(fn GetMyNumber
  (params (Pawn :type Pawn%20Object%20Reference))
  (bind _pawnsinline (Variables|Default|GetPawnsInLine))
  (bind _returnvalue (Utilities|Array|FindItem _pawnsinline Pawn))
  (return _returnvalue (>= _returnvalue 0)))