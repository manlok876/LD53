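; BP_Package is a package actor whose look is driven by the Size and Color fields of its PackageInfo.
; The construction script calls UpdateSize, which sets a uniform actor scale for small, medium or large, and UpdateColor, which creates a dynamic instance of M_Basic on the Box and sets its Color parameter.
; The event graph holds only disabled placeholder events, so the actor has no runtime logic of its own.
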(event EventBeginPlay)

(event Collision|EventActorBeginOverlap
  (params (OtherActor :type Actor%20Object%20Reference)))

(event EventTick
  (params (DeltaSeconds :type Float%20%28single-precision%29)))

(fn ConstructionScript
  (CallFunction|UpdateSize)
  (CallFunction|UpdateColor))

(fn UpdateSize
  (Transformation|SetActorScale3D (Math|Conversions|ToVector(Float) (Utilities|Select :Index (.size (Variables|Default|GetPackageInfo)) :NewEnumerator0 0.25 :NewEnumerator1 0.5 :NewEnumerator2 1.0))))

(fn UpdateColor
  (bind _box (Variables|Default|GetBox))
  (Rendering|Material|SetMaterial _box 0 "/Game/Environment/M_Basic.M_Basic")
  (bind _returnvalue (Rendering|Material|CreateDynamicMaterialInstance _box 0 "/Game/Environment/M_Basic.M_Basic" "None" :!class /Script/Engine.PrimitiveComponent))
  (Rendering|Material|SetVectorParameterValue _returnvalue "Color" (Utilities|Select :Index (.color (Variables|Default|GetPackageInfo)) :NewEnumerator0 "(R=1.000000,G=0.000000,B=0.000000,A=1.000000)" :NewEnumerator1 "(R=0.000000,G=1.000000,B=0.000000,A=1.000000)" :NewEnumerator2 "(R=0.000000,G=0.000000,B=1.000000,A=1.000000)" :NewEnumerator3 "(R=1.000000,G=1.000000,B=0.000000,A=1.000000)") :!class /Script/Engine.MaterialInstanceDynamic))