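; BP_PostBox is a resizable open-ended box, a post shelf compartment built from four walls and an overlap zone.
; The construction script calls UpdateSize, which positions and scales the Top, Bottom, Left and Right walls from Width, Height, Depth and WallThickness.
; It also centers OverlapZone vertically and fits its extent to the interior, inset by wall thickness.
; The file holds no overlap or gameplay logic.
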(event Custom|UpdateSize
  (bind _overlapzone (Variables|Default|GetOverlapZone))
  (Utilities|FlowControl|Sequence
    (:then_0
      (Utilities|FlowControl|Sequence ; Update walls
        (:then_0
          (Transformation|SetRelativeTransform (Variables|Default|GetTop) (Math|Transform|MakeTransform (CallFunction|GetTopWallOffset) "0, 0, 0" (CallFunction|GetHorizontalWallsScale)) false true))
        (:then_1
          (Transformation|SetRelativeTransform (Variables|Default|GetBottom) (Math|Transform|MakeTransform (CallFunction|GetBottomWallOffset) "0, 0, 0" (CallFunction|GetHorizontalWallsScale)) false true))
        (:then_2
          (Transformation|SetRelativeTransform (Variables|Default|GetLeft) (Math|Transform|MakeTransform (CallFunction|GetRightWallOffset) "0, 0, 0" (CallFunction|GetVerticalWallsScale)) false true))
        (:then_3
          (Transformation|SetRelativeTransform (Variables|Default|GetRight) (Math|Transform|MakeTransform (CallFunction|GetLeftWallOffset) "0, 0, 0" (CallFunction|GetVerticalWallsScale)) false true))))
    (:then_1
      (Transformation|SetRelativeLocation _overlapzone (Math|Vector|MakeVector 0.0 0.0 (/ (Variables|Box|GetHeight) 2.0)) false true)
      (Components|Box|SetBoxExtent _overlapzone (CallFunction|GetOverlapExtent) true))))

(event EventBeginPlay)

(event Collision|EventActorBeginOverlap
  (params (OtherActor :type Actor%20Object%20Reference)))

(event EventTick
  (params (DeltaSeconds :type Float%20%28single-precision%29)))

(fn ConstructionScript
  (CallFunction|UpdateSize))

(fn GetOverlapExtent
  (return (- (/ (Math|Vector|MakeVector (Variables|Box|GetDepth) (Variables|Box|GetWidth) (Variables|Box|GetHeight)) 2.0) (Variables|Box|GetWallThickness))))

(fn GetVerticalWallsScale
  (return (/ (Math|Vector|MakeVector (Variables|Box|GetDepth) (Variables|Box|GetWallThickness) (Variables|Box|GetHeight)) 1e+02)))

(fn GetHorizontalWallsScale
  (return (/ (Math|Vector|MakeVector (Variables|Box|GetDepth) (Variables|Box|GetWidth) (Variables|Box|GetWallThickness)) 1e+02)))

(fn GetRightWallOffset
  (return (/ (Math|Vector|MakeVector 0.0 (- (Variables|Box|GetWidth) (Variables|Box|GetWallThickness)) (Variables|Box|GetHeight)) 2.0)))

(fn GetTopWallOffset
  (return (Math|Vector|MakeVector 0.0 0.0 (- (Variables|Box|GetHeight) (/ (Variables|Box|GetWallThickness) 2.0)))))

(fn GetLeftWallOffset
  (return (/ (Math|Vector|MakeVector 0.0 (* -1 (- (Variables|Box|GetWidth) (Variables|Box|GetWallThickness))) (Variables|Box|GetHeight)) 2.0)))

(fn GetBottomWallOffset
  (return (Math|Vector|MakeVector 0.0 0.0 (/ (Variables|Box|GetWallThickness) 2.0))))