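; BP_PostShelf is a shelf actor that generates a grid of BP_PostBox actors from row, column and box-size settings.
; Each box spawns at a computed offset, receives an ID from the shelf ID and its coordinates, then attaches with relative rules so that offset becomes shelf-local.
; InverseDirection flips columns between right and left.
; E_RecreateBoxes and E_ClearBoxes wrap rebuilding and deleting the tracked boxes; BeginPlay and construction create nothing.
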(event Custom|DeleteBoxes
  (bind _createdboxes (Variables|Default|GetCreatedBoxes))
  (for _array_element _createdboxes
    (Actor|DestroyActor _array_element))
  (Utilities|Array|Clear _createdboxes))

(event Custom|CreateBoxes
  (if (not (Shelf|HasAnyBoxes))
    (for _index (range 1 (Variables|Shelf|GetRows))
      (for _index_2 (range 1 (Variables|Shelf|GetColumns))
        (bind _returnvalue (Game|SpawnActorfromClass "/Game/PostObjects/Shelves/BP_PostBox.BP_PostBox_C" (Math|Conversions|ToTransform(Vector) (CallFunction|GetBoxOffset (Utilities|Struct|MakeFShelfCoords _index _index_2))) "Undefined" 0 (Variables|Shelf|GetBoxHeight) (Variables|Shelf|GetBoxWidth) (Variables|Shelf|GetBoxDepth) 0))
        (Variables|/Game/PostObjects/Shelves/BP_PostBox.BP_PostBox_C|SetCoords _returnvalue (Utilities|Struct|MakeFPostBoxID (Variables|Shelf|GetShelfID) (Utilities|Struct|MakeFShelfCoords _index _index_2)))
        (Utilities|Array|Add (Variables|Default|GetCreatedBoxes) _returnvalue)
        (Transformation|AttachActorToActor _returnvalue self "None" "KeepRelative" "KeepRelative" "KeepRelative" true)))))

(event Custom|RecreateBoxes
  (Utilities|FlowControl|Sequence
    (:then_0
      (CallFunction|DeleteBoxes))
    (:then_1
      (CallFunction|CreateBoxes))))

(event EventBeginPlay)

(event Collision|EventActorBeginOverlap
  (params (OtherActor :type Actor%20Object%20Reference)))

(event EventTick
  (params (DeltaSeconds :type Float%20%28single-precision%29)))

(fn ConstructionScript)

(fn HasAnyBoxes
  (return (Utilities|Array|IsNotEmpty (Variables|Default|GetCreatedBoxes))))

(fn GetBoxOffset
  (params (BoxCoords :type F%20Shelf%20Coords%20Structure%20%28by%20ref%29))
  (bind (_row _column) (Utilities|Struct|BreakFShelfCoords BoxCoords))
  (bind _returnvalue (CallFunction|GetRowDirection))
  (return (+ (* (- _row 1) (Variables|Shelf|GetBoxHeight) (Math|Vector|VectorUp)) (* (- _column 1) (Variables|Shelf|GetBoxWidth) _returnvalue) (* _returnvalue (/ (Variables|Shelf|GetBoxWidth) 2.0)))))

(fn ERecreateBoxes
  (CallFunction|RecreateBoxes))

(fn EClearBoxes
  (CallFunction|DeleteBoxes))

(fn GetRowDirection
  (return (select (Variables|Shelf|GetInverseDirection) (Class|KismetMathLibrary|VectorLeft) (Class|KismetMathLibrary|VectorRight))))